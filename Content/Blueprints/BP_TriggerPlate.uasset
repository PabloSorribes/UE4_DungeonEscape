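; BP_TriggerPlate is a weight-sensitive pressure plate that opens and closes a linked BP_MovingWall.
; Trigger overlaps add or subtract each actor's GetWeightMessage value, clamping the total at zero on exit.
; Reaching RequiredWeight opens the wall and turns the plate green; an exit leaving less closes it and turns it red.
; On BeginPlay, an unset MovingWall falls back to the first one found in the level.
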(event `self.ReceiveBeginPlay`
  (`/Engine/EditorBlueprintResources/StandardMacros.IsValid` (`self.MovingWall`)
    (:`Is Not Valid`
      (bind _outactors (`GameplayStatics.GetAllActorsOfClass` "/Game/Blueprints/BP_MovingWall.BP_MovingWall_C"))
      (set `self.MovingWall` (`|GetArrayItem` _outactors))
      (`self.ChangeMaterial` "/Game/Materials/M_RedColor.M_RedColor"))))

(event `self.ResetTrap`
  (`/Game/Blueprints/BP_MovingWall.OpenDoor` (`self.MovingWall`))
  (set `self.isTrapTriggered` false)
  (`self.ChangeMaterial` "/Game/Materials/M_GreenColor.M_GreenColor"))

(event `self.TriggerTrap`
  (`/Game/Blueprints/BP_MovingWall.CloseDoor` (`self.MovingWall`))
  (set `self.isTrapTriggered` true)
  (`self.ChangeMaterial` "/Game/Materials/M_RedColor.M_RedColor"))

(event `self.Trigger.OnComponentBeginOverlap`
  (params (OverlappedComponent :type "PrimitiveComponent Object Reference") (OtherActor :type "Actor Object Reference") (OtherComp :type "PrimitiveComponent Object Reference") (OtherBodyIndex :type Integer) (bFromSweep :type Boolean) (SweepResult :type "HitResult Structure (by ref)"))
  (bind _weight (message `/Game/Blueprints/Interfaces/BPI_Weight.GetWeight` OtherActor))
  (bind _output_get (set `self.CurrentWeight` (+ (`self.CurrentWeight`) _weight)))
  (if (>= _output_get (`self.RequiredWeight`))
    (`self.ResetTrap`)))

(event `self.Trigger.OnComponentEndOverlap`
  (params (OverlappedComponent :type "PrimitiveComponent Object Reference") (OtherActor :type "Actor Object Reference") (OtherComp :type "PrimitiveComponent Object Reference") (OtherBodyIndex :type Integer))
  (bind _weight (message `/Game/Blueprints/Interfaces/BPI_Weight.GetWeight` OtherActor))
  (bind _output_get (set `self.CurrentWeight` (- (`self.CurrentWeight`) _weight)))
  (if (< _output_get 0.0)
    (set `self.CurrentWeight` 0.0))
  (if (< _output_get (`self.RequiredWeight`))
    (`self.TriggerTrap`)))

(event `ChangeMaterial`
  (params (`Material to change` :type "MaterialInstance Object Reference"))
  (`PrimitiveComponent.SetMaterial` (`self.Plate`) 0 `Material to change`))

(fn `UserConstructionScript`)