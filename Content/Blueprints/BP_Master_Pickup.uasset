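; BP_Master_Pickup is a base pickup actor that a BP_CharacterPawn can carry and drop.
; Pickup turns off mesh physics, limits collision to queries, snaps DefaultMesh to the pawn's HoldingPoint, and returns itself with a success flag.
; Drop re-enables physics and full collision, but calls detach on DefaultSceneRoot rather than on the attached DefaultMesh, then returns itself.
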(fn `Drop`
  (returns (myType :type "/Game/Blueprints/BP_Master_Pickup Object Reference"))
  (bind _defaultmesh (`self.DefaultMesh`))
  (`PrimitiveComponent.SetSimulatePhysics` _defaultmesh true)
  (`PrimitiveComponent.SetCollisionEnabled` _defaultmesh "QueryAndPhysics")
  (`SceneComponent.K2_DetachFromComponent` (`self.DefaultSceneRoot`) "KeepRelative" "KeepRelative" "KeepRelative" true)
  (return self))

(fn `Pickup`
  (params (actorThatPicksUp :type "Character Object Reference"))
  (returns (pickedUpObject :type "/Game/Blueprints/BP_Master_Pickup Object Reference") (onPickupSuccess :type Boolean))
  (bind _defaultmesh (`self.DefaultMesh`))
  (`PrimitiveComponent.SetSimulatePhysics` _defaultmesh false)
  (`PrimitiveComponent.SetCollisionEnabled` _defaultmesh "QueryOnly")
  (`SceneComponent.K2_AttachToComponent` (`self.DefaultMesh`) (`/Game/Blueprints/MainScripts/BP_CharacterPawn.HoldingPoint` (cast `/Game/Blueprints/MainScripts/BP_CharacterPawn` actorThatPicksUp :!pure true)) "None" "SnapToTarget" "SnapToTarget" "KeepRelative" true)
  (return self true))

(fn `UserConstructionScript`)