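; BP_MovingWall is a wall that slides between open and closed positions, starting open and closing when something overlaps its trigger.
; OpenDoor and CloseDoor each stop the opposing timeline and restart their own, though only CloseDoor is called here.
; LerpObject moves WallArrow from its current location each update, compounding the timeline alpha into an eased motion.
; Keys 8 and 9 play and reverse an alternative tutorial timeline offset from the initial position.
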(event `self.ReceiveBeginPlay`
  ;[1 1 1] Set start position to OpenPosition by default
  (`SceneComponent.K2_SetRelativeLocation` (`self.WallArrow`) (`self.openPosition`) false false)
  (set `self.initialPosition` (`SceneComponent.RelativeLocation` (`self.WallArrow`))))

(event `self.Trigger.OnComponentBeginOverlap`
  (params (OverlappedComponent :type "PrimitiveComponent Object Reference") (OtherActor :type "Actor Object Reference") (OtherComp :type "PrimitiveComponent Object Reference") (OtherBodyIndex :type Integer) (bFromSweep :type Boolean) (SweepResult :type "HitResult Structure (by ref)"))
  (`self.CloseDoor`))

(event `OpenDoor`
  ;[1 1 1] Open
  (`|ExecutionSequence`
    (:`then_0`
      ;[1 1 1] Close
      (bind (_direction _value) (`Timeline|Timeline_Closed` :!via `Stop` :!label _label)
        (:`Update`
          (`self.LerpObject` (`SceneComponent.RelativeLocation` (`self.WallArrow`)) (`self.closedPosition`) _value (`self.WallArrow`)))))
    (:`then_1`
      (bind (_direction_2 _value_2) (`Timeline|Timeline_Open` :!via `PlayFromStart` :!label _label_2)
        (:`Update`
          (`self.LerpObject` (`SceneComponent.RelativeLocation` (`self.WallArrow`)) (`self.openPosition`) _value_2 (`self.WallArrow`)))))))

(event `CloseDoor`
  ;[1 1 1] Close
  (`|ExecutionSequence`
    (:`then_0`
      (goto _label_2 :!via `Stop`))
    (:`then_1`
      (goto _label :!via `PlayFromStart`))))

(event `Key|Eight`
  (params (Key :type "Key Structure"))
  (:`Pressed`
    ;[1 1 1] Tutorial lerp (not as nice feeling as our shitty one)
    (bind (_direction _new_vector_position) (`Timeline|Tutorial Timeline` :!label _label_3)
      (:`Update`
        (`self.LerpObject` (`SceneComponent.RelativeLocation` (`self.WallArrow`)) (+ (* _new_vector_position (`self.modificationInterval`)) (`self.initialPosition`)) (.z _new_vector_position) (`self.WallArrow`))))))

(event `Key|Nine`
  (params (Key :type "Key Structure"))
  (:`Pressed`
    (goto _label_3 :!via `Reverse`)))

(fn `LerpObject`
  (params (CurrentPosition :type "Vector Structure") (TargetPosition :type "Vector Structure") (Alpha :type "Float (double-precision)") (ObjectToMove :type "SceneComponent Object Reference"))
  (`SceneComponent.K2_SetRelativeLocation` ObjectToMove (`KismetMathLibrary.VLerp` CurrentPosition TargetPosition Alpha) false false))

(fn `UserConstructionScript`)