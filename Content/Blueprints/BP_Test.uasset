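; BP_Test is a scratch actor Blueprint of practice snippets with no complete gameplay behavior.
; Its MoveShit event clears an empty timer handle and calls Set Timer by Event on itself with zero time.
; Disconnected nodes experiment with material changes, casts, wall interpolation and printing, but never execute.
; Pickup only prints a message, while Drop and the construction script are empty.
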(event `MoveShit`
  ;[1 1 1] Timer stuff (ask teacher)
  (`KismetSystemLibrary.K2_ClearAndInvalidateTimerHandle` (make `TimerHandle`))
  (`KismetSystemLibrary.K2_SetTimerDelegate` (delegate `MoveShit`)))

(fn `Drop`
  (returns (myType :type "/Game/Blueprints/BP_Master_Pickup Object Reference"))
  (return null))

(fn `Pickup`
  (params (actorThatPicksUp :type "Character Object Reference"))
  (`KismetSystemLibrary.PrintString` "Im picking up stuff"))

(fn `UserConstructionScript`)