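; BPC_PlayerController is the player controller that forwards input to the active BP_CharacterPawn and handles spawning a new one.
; On BeginPlay it caches the possessed pawn and the first PlayerStart, printing a warning if none exists.
; Input actions drive ragdoll toggling, pickup/drop, throwing and sprinting.
; Hard-wired number keys kill the pawn or spawn and possess a fresh one at the PlayerStart location.
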(event `self.ReceiveBeginPlay`
  (set `self.ActivePlayerCharacter` (cast `/Game/Blueprints/MainScripts/BP_CharacterPawn` (`GameplayStatics.GetPlayerPawn` 0) :!pure true))
  (bind _outactors (`GameplayStatics.GetAllActorsOfClass` "/Script/Engine.PlayerStart"))
  (bind _output (`|GetArrayItem` _outactors))
  (`/Engine/EditorBlueprintResources/StandardMacros.IsValid` _output
    (:`Is Valid`
      (set `self.PlayerStart` _output))
    (:`Is Not Valid`
      (`KismetSystemLibrary.PrintString` "No PlayerStart-object added to the scene"))))

(event `InputAction|ToggleRagdoll`
  (params (Key :type "Key Structure"))
  (bind _activeplayercharacter (`self.ActivePlayerCharacter`))
  (:`Pressed`
    (`/Engine/EditorBlueprintResources/StandardMacros.FlipFlop`
      (:`A`
        (`/Game/Blueprints/MainScripts/BP_CharacterPawn.ActivateRagdoll` _activeplayercharacter))
      (:`B`
        (`/Game/Blueprints/MainScripts/BP_CharacterPawn.DeActivateRagdoll` _activeplayercharacter)))))

(event `InputAction|Use`
  (params (Key :type "Key Structure"))
  (:`Pressed`
    (`/Game/Blueprints/MainScripts/BP_CharacterPawn.Pickup/Drop` (`self.ActivePlayerCharacter`))))

(event `InputAction|SpecialAction`
  (params (Key :type "Key Structure"))
  (:`Pressed`
    (`/Game/Blueprints/MainScripts/BP_CharacterPawn.Throw` (`self.ActivePlayerCharacter`))))

(event `InputAction|ToggleSprint`
  (params (Key :type "Key Structure"))
  (bind _activeplayercharacter (`self.ActivePlayerCharacter`))
  (:`Pressed`
    (`/Game/Blueprints/MainScripts/BP_CharacterPawn.Sprint` _activeplayercharacter))
  (:`Released`
    (`/Game/Blueprints/MainScripts/BP_CharacterPawn.Walk` _activeplayercharacter)))

(event `Key|Two`
  (params (Key :type "Key Structure"))
  (:`Pressed`
    (`/Game/Blueprints/MainScripts/BP_CharacterPawn.KillPlayer` (`self.ActivePlayerCharacter`) true)))

(event `Key|Three`
  (params (Key :type "Key Structure"))
  (:`Pressed`
    (`self.SpawnPlayer`)))

(event `SpawnPlayer`
  (bind _returnvalue (`|SpawnActorFromClass` "/Game/Blueprints/MainScripts/BP_CharacterPawn.BP_CharacterPawn_C" (`KismetMathLibrary.Conv_VectorToTransform` (`self.K2_GetActorLocation` (`self.PlayerStart`))) "Undefined" "OverrideRootScale" null null))
  (bind _output_get (set `self.ActivePlayerCharacter` _returnvalue))
  (`self.Possess` _output_get))

(fn `UserConstructionScript`)