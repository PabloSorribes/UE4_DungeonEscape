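; BP_CharacterPawn is the player character, handling sprint, death, ragdoll, and carrying and throwing objects.
; Death sets IsDead on BPC_PlayerController, optionally ragdolls the whole body with a detached camera boom, then explodes and destroys the pawn.
; A separate toggleable partial ragdoll drives selected limb and neck bones through a macro.
; Pickup uses a forward capsule trace and BPI_Pickupable messages; throwing drops the object and impulses it along camera forward.
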(event `self.ReceiveBeginPlay`
  ;[1 1 1] Begin Play: Set to alive
  (bind _asbpc_player_controller (cast `/Game/Blueprints/MainScripts/BPC_PlayerController` (`GameplayStatics.GetPlayerController` 0)))
  (set `/Game/Blueprints/MainScripts/BPC_PlayerController.isDead` false _asbpc_player_controller))

(event `KillPlayer`
  (params (RagdollOnDeath :type Boolean))
  ;[1 1 1] Death action
  (bind _asbpc_player_controller (cast `/Game/Blueprints/MainScripts/BPC_PlayerController` (`GameplayStatics.GetPlayerController` 0)))
  (set `/Game/Blueprints/MainScripts/BPC_PlayerController.isDead` true _asbpc_player_controller)
  (if RagdollOnDeath
    (`self.RagdollWholePlayer`)
    (`KismetSystemLibrary.Delay` 2.0)
    (`self.OnPlayerDeath`)
    (else
      (`self.OnPlayerDeath`))))

(event `RagdollWholePlayer`
  (bind _mesh (`self.Mesh`))
  ;[1 1 1] Death action
  (`PrimitiveComponent.SetSimulatePhysics` _mesh true)
  (`PrimitiveComponent.SetCollisionObjectType` _mesh "ECC_PhysicsBody")
  (`PrimitiveComponent.SetCollisionEnabled` (`self.CapsuleComponent`) "NoCollision")
  (`SceneComponent.K2_DetachFromComponent` (`self.CameraBoom`) "KeepWorld" "KeepWorld" "KeepWorld" true))

(event `OnPlayerDeath`
  (bind _returnvalue_location (`KismetMathLibrary.BreakTransform` (`self.GetTransform` self)))
  ;[1 1 1] Death action
  (`GameplayStatics.SpawnEmitterAtLocation` "/Game/StarterContent/Particles/P_Explosion.P_Explosion" _returnvalue_location)
  (`self.K2_DestroyActor`))

(event `Sprint`
  ;[1 1 1] Sprint / Walk
  (set `CharacterMovementComponent.MaxWalkSpeed` 1500.0 (`self.CharacterMovement`))
  (set `self.IsSprinting` true))

(event `Walk`
  ;[1 1 1] Sprint / Walk
  (set `CharacterMovementComponent.MaxWalkSpeed` 600.0 (`self.CharacterMovement`))
  (set `self.IsSprinting` false))

(event `ActivateRagdoll`
  (bind _mesh (`self.Mesh`))
  ;[1 1 1] Ragdoll
  (`/Game/Blueprints/Helpers/_MacroLibrary.Macro_ActivateRagdoll` _mesh (`self.LegPart`) true)
  (`/Game/Blueprints/Helpers/_MacroLibrary.Macro_ActivateRagdoll` _mesh "thigh_l" true)
  (`/Game/Blueprints/Helpers/_MacroLibrary.Macro_ActivateRagdoll` (`self.Mesh`) (`self.ArmPart`) true)
  (`/Game/Blueprints/Helpers/_MacroLibrary.Macro_ActivateRagdoll` (`self.Mesh`) "neck_01" true))

(event `DeActivateRagdoll`
  (bind _mesh (`self.Mesh`))
  ;[1 1 1] Ragdoll
  (`/Game/Blueprints/Helpers/_MacroLibrary.Macro_ActivateRagdoll` _mesh (`self.LegPart`))
  (`/Game/Blueprints/Helpers/_MacroLibrary.Macro_ActivateRagdoll` _mesh "thigh_l")
  (`/Game/Blueprints/Helpers/_MacroLibrary.Macro_ActivateRagdoll` (`self.Mesh`) (`self.ArmPart`))
  (`/Game/Blueprints/Helpers/_MacroLibrary.Macro_ActivateRagdoll` (`self.Mesh`) "neck_01"))

(event `Pickup/Drop`
  ;[1 1 1] Pickup / Drop
  (if (`self.IsHolding`)
    (`self.DropObject`)
    (else
      (`self.PickupObject`))))

(event `Throw`
  ;[1 1 1] Throw
  (if (`self.IsHolding`)
    (`self.ThrowObject`)))

(fn `DropObject`
  (message `/Game/Blueprints/Interfaces/BPI_Pickupable.Drop` (`self.LastPickedUpObject`))
  (set `self.IsHolding` false))

(fn `GetWeight`
  (returns (Weight :type "Float (double-precision)"))
  (return (`self.PlayerWeight`)))

(fn `PickupObject`
  (bind _capsulecomponent (`self.CapsuleComponent`))
  (bind _returnvalue (`SceneComponent.K2_GetComponentLocation` _capsulecomponent))
  (bind (_outhit _returnvalue_2) (`KismetSystemLibrary.CapsuleTraceSingle` _returnvalue (+ _returnvalue (* (`SceneComponent.GetForwardVector` _capsulecomponent) (`self.PickupDistance`))) 50.0 0.0 "TraceTypeQuery1"))
  (bind (_bblockinghit _binitialoverlap _time _distance _location _impactpoint _normal _impactnormal _physmat _hitactor) (`GameplayStatics.BreakHitResult` _outhit))
  (if (and _returnvalue_2 (`KismetSystemLibrary.DoesImplementInterface` _hitactor "/Game/Blueprints/Interfaces/BPI_Pickupable.BPI_Pickupable_C"))
    (bind (_pickedupobject _onpickupsuccess) (message `/Game/Blueprints/Interfaces/BPI_Pickupable.Pickup` _hitactor self))
    (if _onpickupsuccess
      (set `self.LastPickedUpObject` _pickedupobject)
      (set `self.IsHolding` true))
    (else
      (`KismetSystemLibrary.PrintString` "Object is not Pickupable"))))

(fn `ThrowObject`
  (`self.DropObject`)
  (`PrimitiveComponent.AddImpulse` (`/Game/Blueprints/BP_Master_Pickup.DefaultMesh` (`self.LastPickedUpObject`)) (* (`SceneComponent.GetForwardVector` (`self.FollowCamera`)) (`self.ThrowMultiplication`)) "None" true))

(fn `UserConstructionScript`
  (`parent.UserConstructionScript`))